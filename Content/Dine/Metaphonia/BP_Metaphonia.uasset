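; Metaphonia is an AI-moved pawn that can follow the player character around.
; BeginPlay caches the BP_Player reference, and the FollowPlayer event, started from outside this graph, runs while its flag of the same name is set.
; It issues AI MoveTo toward the player, or toward itself to hold position when within 50 units.
; The event re-triggers itself after a short delay, forming a polling loop.
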(event Custom|Follow%20Player
  (if (Variables|Default|GetFollowPlayer?)
    (if (>= (Transformation|GetDistanceTo (Variables|Default|GetChar%20Ref)) 5e+01)
      (AI|AIMoveTo self "0, 0, 0" (Variables|Default|GetChar%20Ref) 5.0 false
        (:then
          _))
      (else
        (AI|AIMoveTo self "0, 0, 0" self 5.0 false
          (:then
            _))))
    (Utilities|FlowControl|Delay 0.2)
    (CallFunction|FollowPlayer)))

(event EventBeginPlay
  (bind _asbp_player (Utilities|Casting|CastToBP_Player (Game|GetPlayerCharacter 0)))
  (Variables|Default|SetChar%20Ref _asbp_player))

(fn ConstructionScript)